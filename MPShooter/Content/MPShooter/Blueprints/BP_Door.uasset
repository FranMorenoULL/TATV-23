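; BP_Door is a hinged door that opens when enough ShooterPawns stand in its detection box and closes when the count drops below the minimum.
; On the authority only, overlap events update the player count and toggle the open state.
; Opening and closing play or reverse a timeline that drives the hinge's yaw, and tint the door's dynamic material green or red.
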(event OnComponentBeginOverlap(DetectionBox)
  (params (OverlappedComponent :type Primitive%20Component%20Object%20Reference) (OtherActor :type Actor%20Object%20Reference) (OtherComp :type Primitive%20Component%20Object%20Reference) (OtherBodyIndex :type Integer) (bFromSweep :type Boolean) (SweepResult :type Hit%20Result%20Structure%20%28by%20ref%29))
  (Networking|SwitchHasAuthority
    (:Authority
      (Utilities|Casting|CastToShooterPawn OtherActor)
      (bind _result (Math|Integer|IncrementInt (Variables|Door|GetPlayersCount))
        (:%20%20
          (if (and (>= _result (Variables|Door|GetMinPlayersCountToOpen)) (not (Variables|Door|GetbIsOpen)))
            (Development|PrintString "Hello")
            (Variables|Door|SetbIsOpen true)
            (CallFunction|OpenDoor)))))))

(event OnComponentEndOverlap(DetectionBox)
  (params (OverlappedComponent :type Primitive%20Component%20Object%20Reference) (OtherActor :type Actor%20Object%20Reference) (OtherComp :type Primitive%20Component%20Object%20Reference) (OtherBodyIndex :type Integer))
  (Networking|SwitchHasAuthority
    (:Authority
      (Utilities|Casting|CastToShooterPawn OtherActor)
      (bind _result (Math|Integer|DecrementInt (Variables|Door|GetPlayersCount))
        (:%20%20
          (if (and (< _result (Variables|Door|GetMinPlayersCountToOpen)) (Variables|Door|GetbIsOpen))
            (Development|PrintString "Bye")
            (Variables|Door|SetbIsOpen false)
            (CallFunction|CloseDoor)))))))

(event Custom|OpenDoor
  (bind _hinge (Variables|Default|GetHinge))
  (bind _relativerotation (Variables|/Script/Engine.SceneComponent|GetRelativeRotation _hinge))
  (Rendering|Material|SetVectorParameterValue (Variables|Door|GetDoorMaterial) "BaseColor" "(R=0.000000,G=1.000000,B=0.000000,A=1.000000)" :!class /Script/Engine.MaterialInstanceDynamic)
  (bind _yaw (Timeline|Timeline Play)
    (:Update
      (Transformation|SetRelativeRotation _hinge (Math|Rotator|MakeRotator (.roll _relativerotation) (.pitch _relativerotation) _yaw) false false))))

(event Custom|CloseDoor
  (bind _hinge (Variables|Default|GetHinge))
  (bind _relativerotation (Variables|/Script/Engine.SceneComponent|GetRelativeRotation _hinge))
  (Rendering|Material|SetVectorParameterValue (Variables|Door|GetDoorMaterial) "BaseColor" "(R=1.000000,G=0.000000,B=0.000000,A=1.000000)" :!class /Script/Engine.MaterialInstanceDynamic)
  (bind _yaw (Timeline|Timeline Reverse)
    (:Update
      (Transformation|SetRelativeRotation _hinge (Math|Rotator|MakeRotator (.roll _relativerotation) (.pitch _relativerotation) _yaw) false false))))

(event EventBeginPlay
  (bind _staticmesh (Variables|Default|GetStaticMesh))
  (bind _returnvalue (Rendering|Material|CreateDynamicMaterialInstance _staticmesh 0 "/Game/MPShooter/Materials/Door/M_Door.M_Door" "None" :!class /Script/Engine.PrimitiveComponent))
  (bind _output_get (Variables|Door|SetDoorMaterial _returnvalue))
  (Rendering|Material|SetMaterial _staticmesh 0 _output_get))

(fn ConstructionScript)