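; BP_Weapon is a weapon actor in a multiplayer tutorial that spawns bullets and firing effects.
; SpawnBullet casts its owner to Pawn and spawns a BP_Bullet just ahead of the weapon, facing its rotation, with the weapon as Owner and that pawn as Instigator.
; FireFX is a separate event that spawns a Niagara fire effect at the same offset.
; The FireBullet function is an empty stub.
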(event Custom|Spawn%20Bullet
  (bind _aspawn (Utilities|Casting|CastToPawn (Components|GetOwner)))
  (Game|SpawnActorfromClass "/Game/MultiplayerTutorial/Blueprints/BP_Bullet.BP_Bullet_C" (Math|Transform|MakeTransform (+ (* (Transformation|GetActorForwardVector) 5e+01) (Transformation|GetActorLocation)) (Transformation|GetActorRotation) "1.000000,1.000000,1.000000") "Undefined" self _aspawn))

(event Custom|FireFX
  (Niagara|SpawnSystematLocation "/Game/FX/NE_Fire_System.NE_Fire_System" (+ (* (Transformation|GetActorForwardVector) 5e+01) (Transformation|GetActorLocation))))

(fn ConstructionScript)

(fn FireBullet)