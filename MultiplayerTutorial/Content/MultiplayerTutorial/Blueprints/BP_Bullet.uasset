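; BP_Bullet is a projectile from a multiplayer tutorial that deals area damage when its sphere component hits something.
; On impact it overlaps nearby pawns and calls AffectedByShot on third-person characters, passing damage and an upward-biased impulse away from the bullet.
; Only the authority calls Explode, which spawns a Niagara burst at the impact location, and the bullet then destroys itself.
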(event OnComponentHit(Sphere)
  (params (HitComponent :type Primitive%20Component%20Object%20Reference) (OtherActor :type Actor%20Object%20Reference) (OtherComp :type Primitive%20Component%20Object%20Reference) (NormalImpulse :type Vector :default "0, 0, 0") (Hit :type Hit%20Result%20Structure%20%28by%20ref%29))
  ;[1 1 1] Projectile Impact
  (bind _outactors (Collision|SphereOverlapActors (Transformation|GetActorLocation) 1e+02 (Utilities|Array|MakeArray "ObjectTypeQuery3") 0))
  (for _array_element _outactors
    (bind _asbp_third_person_character (Utilities|Casting|CastToBP_ThirdPersonCharacter _array_element))
    (Default|AffectedbyShot _asbp_third_person_character (Variables|Default|GetDamage) (* (Variables|Default|GetImpulseEffect) (Math|Vector|Normalize (+ (Math|Vector|GetUnitDirection(Vector) (Transformation|GetActorLocation) (Transformation|GetActorLocation _array_element)) "0.000000,0.000000,1.000000")))))
  (Networking|SwitchHasAuthority
    (:Authority
      (CallFunction|Explode))
    (:Remote
      _))
  (Actor|DestroyActor))

(event Custom|Explode
  (Niagara|SpawnSystematLocation "/Game/FX/NE_Burst_System.NE_Burst_System" (Transformation|GetActorLocation)))

(fn ConstructionScript)